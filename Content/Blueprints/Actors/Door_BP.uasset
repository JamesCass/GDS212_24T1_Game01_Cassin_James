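; Interactable hinged door that swings open and closed by 90 degrees of yaw.
; A box collider sends interface messages to overlapping actors when they enter, passing itself, and when they exit.
; DoMyInteraction uses a FlipFlop to alternately add and subtract 90 from TargetYaw, which starts at the initial yaw.
; Tick lerps the root's world yaw halfway to that target each frame, giving frame-rate-dependent easing.
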(event OnComponentBeginOverlap(Box)
  (params (OverlappedComponent :type Primitive%20Component%20Object%20Reference) (OtherActor :type Actor%20Object%20Reference) (OtherComp :type Primitive%20Component%20Object%20Reference) (OtherBodyIndex :type Integer) (bFromSweep :type Boolean) (SweepResult :type Hit%20Result%20Structure%20%28by%20ref%29))
  ;[1 1 1] collider to interact with door
  (Class|InteractInterface|InteractAreaEntered(Message) OtherActor self))

(event OnComponentEndOverlap(Box)
  (params (OverlappedComponent :type Primitive%20Component%20Object%20Reference) (OtherActor :type Actor%20Object%20Reference) (OtherComp :type Primitive%20Component%20Object%20Reference) (OtherBodyIndex :type Integer))
  ;[1 1 1] collider to interact with door
  (Class|InteractInterface|InteractAreaExited(Message) OtherActor))

(event EventDoMyInteraction
  ;[1 1 1] sets door open / closed position
  (Utilities|FlowControl|FlipFlop
    (:A
      (Variables|Default|SetTargetYaw (+ (Variables|Default|GetTargetYaw) 9e+01)))
    (:B
      (Variables|Default|SetTargetYaw (- (Variables|Default|GetTargetYaw) 9e+01)))))

(event EventBeginPlay
  ;[1 1 1] sets door closed position
  (Variables|Default|SetTargetYaw (.yaw (Transformation|GetWorldRotation (Variables|Default|GetDefaultSceneRoot)))))

(event EventTick
  (params (DeltaSeconds :type Float%20%28single-precision%29))
  ;[1 1 1] Smoothly moves door open / closed
  (Transformation|SetWorldRotation (Variables|Default|GetDefaultSceneRoot) (Math|Rotator|MakeRotator 0.0 0.0 (Math|Float|Lerp (.yaw (Transformation|GetWorldRotation (Variables|Default|GetDefaultSceneRoot))) (Variables|Default|GetTargetYaw) 0.5)) false false))

(fn ConstructionScript)